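; Laser beam actor that damages Cello and toggles Activation Diamonds, bouncing and splitting off surfaces.
; Each tick a line trace sets the beam endpoint and impact effect, tracking the previous actor to deactivate it.
; Splitter actors and Reflective, Splitter or Transparent component tags recursively spawn child lasers up to MaxBounces; Refractive is an empty stub.
; Children respawn only when the hit component or its transform changes, and are destroyed with their parent.
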(event `self.ReceiveBeginPlay`
  (bind _audio (`self.Audio`))
  (`ActorComponent.SetActive` (`self.Laser`) true false)
  (`ActorComponent.SetActive` (`self.Impact`) true false)
  (`GameplayStatics.PlaySoundAtLocation` "/Game/Audio/Sounds/Laser_Start.Laser_Start" (`SceneComponent.K2_GetComponentLocation` (`self.DefaultSceneRoot`)) (struct) 1.0 1.0 0.0 null null null null)
  (`KismetSystemLibrary.Delay` (`SoundBase.Duration` (`AudioComponent.Sound` _audio)))
  (`AudioComponent.SetSound` _audio "/Game/Audio/Sounds/Laser.Laser")
  (`AudioComponent.Play` _audio 0.0))

(event `self.ReceiveTick`
  (params (DeltaSeconds :type "Float (single-precision)"))
  (bind _previous_actor (`self.Previous Actor`))
  (bind _arrow (`self.Arrow`))
  (bind _impact (`self.Impact`))
  (bind _returnvalue (`SceneComponent.K2_GetComponentLocation` _arrow))
  (bind _returnvalue_2 (`SceneComponent.GetForwardVector` _arrow))
  (bind _returnvalue_3 (+ (* _returnvalue_2 (`self.Range`)) _returnvalue))
  (bind _outhit (`KismetSystemLibrary.LineTraceSingle` _returnvalue _returnvalue_3 "TraceTypeQuery2" true (`self.Ignored Actors`)))
  (`FXSystemComponent.SetVectorParameter` (`self.Laser`) "Laser End Point" (`KismetMathLibrary.SelectVector` (`.ImpactPoint` (`GameplayStatics.BreakHitResult` _outhit)) _returnvalue_3 (`GameplayStatics.BreakHitResult` _outhit)))
  (`SceneComponent.SetVisibility` _impact (`GameplayStatics.BreakHitResult` _outhit) false)
  (`|ExecutionSequence`
    (:`then_0`
      (if (`GameplayStatics.BreakHitResult` _outhit)
        (`SceneComponent.K2_SetWorldLocation` _impact (`.ImpactPoint` (`GameplayStatics.BreakHitResult` _outhit)) false false)
        (bind _returnvalue_4 (`KismetSystemLibrary.IsValid` (`.HitActor` (`GameplayStatics.BreakHitResult` _outhit))))
        (if _returnvalue_4
          (`self.Affect Actor` (`.HitActor` (`GameplayStatics.BreakHitResult` _outhit)) true)))
      (if (and (!= (`.HitActor` (`GameplayStatics.BreakHitResult` _outhit)) _previous_actor) (`KismetSystemLibrary.IsValid` _previous_actor))
        (`self.Affect Actor` _previous_actor))
      (if _returnvalue_4
        (set `self.Previous Actor` (`.HitActor` (`GameplayStatics.BreakHitResult` _outhit)))))
    (:`then_1`
      (`self.Alter Laser` (`.HitActor` (`GameplayStatics.BreakHitResult` _outhit)) (`.HitComponent` (`GameplayStatics.BreakHitResult` _outhit)) (`.ImpactPoint` (`GameplayStatics.BreakHitResult` _outhit)) (`.ImpactNormal` (`GameplayStatics.BreakHitResult` _outhit)) _returnvalue_2))))

(event `self.ReceiveDestroyed`
  (`self.Delete Child Lasers`)
  (bind _previous_actor (`self.Previous Actor`)
    (:`then`
      (`self.Affect Actor` _previous_actor))
    (:`else`)))

(fn `Add Child Laser`
  (params (Transform :type "Transform Structure") (`Ignored Actor` :type "Actor Object Reference"))
  (bind _returnvalue (`|SpawnActorFromClass` "Laser_bp_C" Transform "Undefined" "OverrideRootScale" null null))
  (set `/Game/Blueprints/Laser_bp.Bounces` (+ (`self.Bounces`) 1) _returnvalue)
  (if (`KismetSystemLibrary.IsValid` `Ignored Actor`)
    (`KismetArrayLibrary.Array_Add` (`/Game/Blueprints/Laser_bp.Ignored Actors` _returnvalue) `Ignored Actor`))
  (`KismetArrayLibrary.Array_Add` (`self.Child Lasers`) _returnvalue))

(fn `Affect Actor`
  (params (`Target Actor` :type "Actor Object Reference") (Hitting :type Boolean))
  (bind _ascello_bp (cast `/Game/Blueprints/Cello_bp` `Target Actor`)
    (:`then`
      (if Hitting
        (`GameplayStatics.ApplyDamage` _ascello_bp (`self.Damage`))))
    (:`CastFailed`
      (bind _asactivation_diamond_bp (cast `/Game/Blueprints/Activation_Diamond_bp` `Target Actor`))
      (if Hitting
        (`/Game/Blueprints/Activation_Diamond_bp.Activate` _asactivation_diamond_bp)
        (else
          (`/Game/Blueprints/Activation_Diamond_bp.Deactivate` _asactivation_diamond_bp))))))

(fn `Alter Laser`
  (params (`Actor Hit` :type "Actor Object Reference") (`Component Hit` :type "PrimitiveComponent Object Reference") (`Impact Location` :type "Vector Structure") (`Impact Normal` :type "Vector Structure") (`Impact Direction` :type "Vector Structure"))
  (bind (_returnvalue_location _returnvalue_rotation _returnvalue_scale) (`KismetMathLibrary.BreakTransform` (`SceneComponent.K2_GetComponentToWorld` `Component Hit`)))
  (bind _reflected_transform (`self.Get Reflected Transform` `Impact Location` `Impact Normal` `Impact Direction`))
  (bind _componenttags (`ActorComponent.ComponentTags` `Component Hit`))
  (bind (_previous_hit_transform_location _previous_hit_transform_rotation _previous_hit_transform_scale) (break `/Game/Blueprints/TransformStruct` (`self.Previous Hit Transform`)))
  (bind (_returnvalue_location_2 _returnvalue_rotation_2 _returnvalue_scale_2) (`KismetMathLibrary.BreakTransform` (`SceneComponent.K2_GetComponentToWorld` (`self.Laser`))))
  (bind _returnvalue (`KismetMathLibrary.MakeTransform` `Impact Location` _returnvalue_rotation_2 _returnvalue_scale_2))
  (if (and (`KismetSystemLibrary.IsValid` `Component Hit`) (< (`self.Bounces`) (`self.Max Bounces`)))
    (if (or (!= `Component Hit` (`self.Previous Hit`)) (and true (or (!= _returnvalue_location _previous_hit_transform_location :`ErrorTolerance` 0.001) (!= _returnvalue_rotation _previous_hit_transform_rotation :`ErrorTolerance` 0.001) (!= _returnvalue_scale _previous_hit_transform_scale :`ErrorTolerance` 0.001))))
      (`self.Delete Child Lasers`)
      (set `self.Previous Hit` `Component Hit`)
      (`GameplayStatics.PlaySoundAtLocation` "/Game/Audio/Sounds/Laser_Singe.Laser_Singe" `Impact Location` (struct) 1.0 1.0 0.0 null null null null)
      (set `self.Previous Hit Transform` (make `/Game/Blueprints/TransformStruct` _returnvalue_location _returnvalue_rotation _returnvalue_scale))
      (bind _assplitter_bp (cast `/Game/Blueprints/Splitter_bp` `Actor Hit`)
        (:`then`
          (for _array_element (`/Game/Blueprints/Splitter_bp.Get Exit Points` _assplitter_bp)
            (`self.Add Child Laser` _array_element `Actor Hit`)))
        (:`CastFailed`
          (if (`KismetArrayLibrary.Array_Contains` _componenttags "Reflective")
            (`self.Add Child Laser` _reflected_transform `Actor Hit`)
            (elif (`KismetArrayLibrary.Array_Contains` _componenttags "Splitter")
              (`self.Add Child Laser` _returnvalue `Actor Hit`)
              (`self.Add Child Laser` _reflected_transform `Actor Hit`)
              (elif (`KismetArrayLibrary.Array_Contains` _componenttags "Transparent")
                (`self.Add Child Laser` _returnvalue `Actor Hit`)
                (elif (`KismetArrayLibrary.Array_Contains` _componenttags "Refractive")
                  _)))))))
    (else
      (`self.Delete Child Lasers`))))

(fn `Delete Child Lasers`
  (bind _child_lasers (`self.Child Lasers`))
  (for _array_element _child_lasers
    (`self.K2_DestroyActor` _array_element))
  (`KismetArrayLibrary.Array_Clear` _child_lasers))

(fn `Get Reflected Transform`
  (params (`Impact Location` :type "Vector Structure") (`Impact Normal` :type "Vector Structure") (`Impact Direction` :type "Vector Structure"))
  (returns (`Reflected Transform` :type "Transform Structure"))
  (return (`KismetMathLibrary.MakeTransform` `Impact Location` (`KismetMathLibrary.Conv_VectorToRotator` (`KismetMathLibrary.RotateAngleAxis` (* `Impact Direction` -1.0) 180.0 `Impact Normal`)))))

(fn `UserConstructionScript`
  (`FXSystemComponent.SetColorParameter` (`self.Laser`) "Color" (`self.Laser Color`))
  (`FXSystemComponent.SetColorParameter` (`self.Impact`) "Color" (`self.Laser Color`))
  (`AudioComponent.SetSound` (`self.Audio`) "/Game/Audio/Sounds/Laser_Start.Laser_Start"))