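; Health pickup that heals a Cello_bp on overlapping its PickupRange, bypassing the heal cooldown, then destroys itself.
; MagnetRange overlaps maintain a set of target actors, which drives Magnetize every tick while non-empty.
; With positive MagnetStrength, Magnetize enables physics and applies a summed acceleration along vectors pointing from each target toward the pickup (away from targets), weakening linearly with distance across the magnet radius.
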(event `self.Pickup Range.OnComponentBeginOverlap`
  (params (OverlappedComponent :type "PrimitiveComponent Object Reference") (OtherActor :type "Actor Object Reference") (OtherComp :type "PrimitiveComponent Object Reference") (OtherBodyIndex :type Integer) (bFromSweep :type Boolean) (SweepResult :type "HitResult Structure (by ref)"))
  (bind _ascello_bp (cast `/Game/Blueprints/Cello_bp` OtherActor))
  (`/Game/Blueprints/Cello_bp.Heal` _ascello_bp (`self.Heal Amount`) true)
  (`self.K2_DestroyActor`))

(event `self.Magnet Range.OnComponentBeginOverlap`
  (params (OverlappedComponent :type "PrimitiveComponent Object Reference") (OtherActor :type "Actor Object Reference") (OtherComp :type "PrimitiveComponent Object Reference") (OtherBodyIndex :type Integer) (bFromSweep :type Boolean) (SweepResult :type "HitResult Structure (by ref)"))
  (`BlueprintSetLibrary.Set_Add` (`self.Targets`) OtherActor))

(event `self.Magnet Range.OnComponentEndOverlap`
  (params (OverlappedComponent :type "PrimitiveComponent Object Reference") (OtherActor :type "Actor Object Reference") (OtherComp :type "PrimitiveComponent Object Reference") (OtherBodyIndex :type Integer))
  (`BlueprintSetLibrary.Set_Remove` (`self.Targets`) OtherActor))

(event `self.ReceiveTick`
  (params (DeltaSeconds :type "Float (single-precision)"))
  (if (`BlueprintSetLibrary.Set_IsNotEmpty` (`self.Targets`))
    (`self.Magnetize`)))

(fn `Magnetize`
  (locals (`Launch Vector` :type "Vector Structure"))
  (bind _pickup (`self.Pickup`))
  (bind _returnvalue (`SceneComponent.K2_GetComponentLocation` _pickup))
  (if (> (`self.Magnet Strength`) 0.0)
    (`PrimitiveComponent.SetSimulatePhysics` _pickup true)
    (bind _result (`BlueprintSetLibrary.Set_ToArray` (`self.Targets`)))
    (for _array_element _result
      (bind _returnvalue_2 (`self.K2_GetActorLocation` _array_element))
      (set `local.Launch Vector` (+ (* (`KismetMathLibrary.Normal` (- _returnvalue _returnvalue_2)) (- 1.0 (/ (`KismetMathLibrary.Vector_Distance` _returnvalue_2 _returnvalue) (`SphereComponent.SphereRadius` (`self.Magnet Range`)))) (`self.Magnet Strength`)) (`local.Launch Vector`))))
    (`PrimitiveComponent.AddForce` _pickup (`local.Launch Vector`) "None" true)))

(fn `UserConstructionScript`)