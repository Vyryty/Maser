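; An activatable laser actor that switches its beam on or off in response to activators, extending a parent laser Blueprint.
; Activate and Deactivate update a list of activators, then derive the active state from the MinActivators threshold XOR InitialActive, allowing inverted behavior.
; That state drives the visibility and activation of the Laser and Impact components, deletes child lasers when off, and gates the parent's Tick.
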(event `self.ReceiveTick`
  (params (DeltaSeconds :type "Float (single-precision)"))
  (if (`self.Active`)
    (`parent.ReceiveTick` DeltaSeconds)))

(event `/Game/Blueprints/Interaction.Activate`
  (params (Activator :type "Actor Object Reference"))
  (bind _laser (`self.Laser`))
  (bind _activators (`self.Activators`))
  (set `self.Active` true)
  (`BlueprintSetLibrary.Set_Add` _activators Activator)
  (bind _output_get (set `self.Active` (xor (>= (`BlueprintSetLibrary.Set_Length` _activators) (`self.Min Activators`)) (`self.Initial Active`)) :!label _label))
  (`SceneComponent.SetVisibility` _laser _output_get true)
  (`SceneComponent.SetVisibility` (`self.Impact`) _output_get true)
  (`ActorComponent.SetActive` _laser _output_get false)
  (`ActorComponent.SetActive` (`self.Impact`) _output_get false)
  (if (not _output_get)
    (`self.Delete Child Lasers`)))

(event `/Game/Blueprints/Interaction.Deactivate`
  (params (Deactivator :type "Actor Object Reference"))
  (set `self.Active` false)
  (`BlueprintSetLibrary.Set_Remove` (`self.Activators`) Deactivator)
  (goto _label))

(fn `UserConstructionScript`
  (`parent.UserConstructionScript`))