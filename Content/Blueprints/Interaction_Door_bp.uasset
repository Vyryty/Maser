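; Interaction door Blueprint that opens when enough activators trigger it and closes when too few remain.
; Activate and Deactivate add or remove entries in an activator list, then share one check against the minimum activator count.
; Reaching the threshold sets Opened and calls OpenDoor, while dropping below calls CloseDoor unless the door is one-time and has already opened.
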(event `/Game/Blueprints/Interaction.Activate`
  (params (Activator :type "Actor Object Reference"))
  (bind _activators (`self.Activators`))
  (`BlueprintSetLibrary.Set_Add` _activators Activator)
  (if (>= (`BlueprintSetLibrary.Set_Length` _activators) (`self.Min Activators`)) :!label _label
    (set `self.Opened` true)
    (`self.Open Door` false)
    (elif (not (and (`self.One Time`) (`self.Opened`)))
      (`self.Close Door`))))

(event `/Game/Blueprints/Interaction.Deactivate`
  (params (Deactivator :type "Actor Object Reference"))
  (`BlueprintSetLibrary.Set_Remove` (`self.Activators`) Deactivator)
  (goto _label))

(fn `UserConstructionScript`
  (`parent.UserConstructionScript`))