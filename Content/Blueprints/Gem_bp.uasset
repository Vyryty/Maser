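; Gem pickup that bobs up and down and adds one to the gem count of a Cello_bp that touches it.
; The construction script stores the starting location, and the FloatControl timeline lerps the root between it and a point above.
; When the timeline finishes it toggles Rising to alternate between play and reverse.
; Overlapping the Sphere with a Cello_bp calls ChangeGemCount and destroys the gem.
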(event `self.ReceiveBeginPlay`
  (bind _initial_position (`self.Initial Position`))
  (bind _rising (`self.Rising`))
  (if _rising :!label _label
    (bind (_direction _position) (`Timeline|Float Control` :!label _label_2)
      (:`Update`
        (`SceneComponent.K2_SetRelativeLocation` (`self.DefaultSceneRoot`) (`KismetMathLibrary.VLerp` _initial_position (+ _initial_position (0.0 0.0 50.0)) _position) false false))
      (:`Finished`
        (set `self.Rising` (not _rising))
        (goto _label)))
    (else
      (goto _label_2 :!via `Reverse`))))

(event `self.Sphere.OnComponentBeginOverlap`
  (params (OverlappedComponent :type "PrimitiveComponent Object Reference") (OtherActor :type "Actor Object Reference") (OtherComp :type "PrimitiveComponent Object Reference") (OtherBodyIndex :type Integer) (bFromSweep :type Boolean) (SweepResult :type "HitResult Structure (by ref)"))
  (bind _ascello_bp (cast `/Game/Blueprints/Cello_bp` OtherActor))
  (`/Game/Blueprints/Cello_bp.Change Gem Count` _ascello_bp 1)
  (`self.K2_DestroyActor`))

(fn `UserConstructionScript`
  (set `self.Initial Position` (`self.K2_GetActorLocation`)))