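; Push door Blueprint that opens when a component enters its trigger box and closes once the box is clear.
; On overlap, a dot product against the box's forward vector tells OpenDoor which side the component approaches from.
; A Contacts set tracks overlapping components, so CloseDoor runs only when the last one leaves.
; OpenDoor and CloseDoor are called here but defined outside these graphs.
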(event `self.Box_0.OnComponentBeginOverlap`
  (params (OverlappedComponent :type "PrimitiveComponent Object Reference") (OtherActor :type "Actor Object Reference") (OtherComp :type "PrimitiveComponent Object Reference") (OtherBodyIndex :type Integer) (bFromSweep :type Boolean) (SweepResult :type "HitResult Structure (by ref)"))
  (bind _box_0 (`self.Box_0`))
  (`BlueprintSetLibrary.Set_Add` (`self.Contacts`) OtherComp)
  (`self.Open Door` (> (`KismetMathLibrary.Dot_VectorVector` (- (`SceneComponent.K2_GetComponentLocation` _box_0) (`SceneComponent.K2_GetComponentLocation` OtherComp)) (`SceneComponent.GetForwardVector` _box_0)) 0.0)))

(event `self.Box_0.OnComponentEndOverlap`
  (params (OverlappedComponent :type "PrimitiveComponent Object Reference") (OtherActor :type "Actor Object Reference") (OtherComp :type "PrimitiveComponent Object Reference") (OtherBodyIndex :type Integer))
  (bind _contacts (`self.Contacts`))
  (`BlueprintSetLibrary.Set_Remove` _contacts OtherComp)
  (if (`BlueprintSetLibrary.Set_IsEmpty` _contacts)
    (`self.Close Door`)))

(fn `UserConstructionScript`
  (`parent.UserConstructionScript`))