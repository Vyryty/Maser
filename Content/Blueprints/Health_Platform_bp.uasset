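; Health platform that heals Cello_bp actors standing within its capsule.
; Capsule begin and end overlap events add and remove actors in a Targets set.
; Every tick it iterates that set, casts each entry to Cello_bp and calls Heal with HealAmount, leaving the Heal cooldown in effect rather than timing heals itself.
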(event `self.ReceiveTick`
  (params (DeltaSeconds :type "Float (single-precision)"))
  (bind _result (`BlueprintSetLibrary.Set_ToArray` (`self.Targets`)))
  (for _array_element _result
    (bind _ascello_bp (cast `/Game/Blueprints/Cello_bp` _array_element))
    (`/Game/Blueprints/Cello_bp.Heal` _ascello_bp (`self.Heal Amount`) false)))

(event `self.Capsule.OnComponentBeginOverlap`
  (params (OverlappedComponent :type "PrimitiveComponent Object Reference") (OtherActor :type "Actor Object Reference") (OtherComp :type "PrimitiveComponent Object Reference") (OtherBodyIndex :type Integer) (bFromSweep :type Boolean) (SweepResult :type "HitResult Structure (by ref)"))
  (`BlueprintSetLibrary.Set_Add` (`self.Targets`) OtherActor))

(event `self.Capsule.OnComponentEndOverlap`
  (params (OverlappedComponent :type "PrimitiveComponent Object Reference") (OtherActor :type "Actor Object Reference") (OtherComp :type "PrimitiveComponent Object Reference") (OtherBodyIndex :type Integer))
  (`BlueprintSetLibrary.Set_Remove` (`self.Targets`) OtherActor))

(fn `UserConstructionScript`)