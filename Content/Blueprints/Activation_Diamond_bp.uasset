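; Activation diamond that warms up when activated and, once fully charged, triggers its linked Interaction_Door_bp actors.
; A timeline played forward or reversed blends spin, material color, brightness and audio pitch from base values captured in the construction script via a dynamic material.
; Completing warmup applies the active look, plays a gem sound and activates the doors.
; Reversing deactivates them on its first update and silences the audio when finished.
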(event `Activate`
  (bind _audio (`self.Audio`))
  (bind _material (`self.Material`))
  (bind _material_2 (`self.Material`))
  (if (not (`self.Active`))
    (set `self.Active` true)
    (bind (_direction _warmup_time) (`Timeline|Diamond Control` :!label _label)
      (:`Update`
        (set `RotatingMovementComponent.RotationRate` (`KismetMathLibrary.RLerp` (`self.Base Rotation`) (`self.Active Rotation`) _warmup_time) (`self.RotatingMovement`))
        (`MaterialInstanceDynamic.SetVectorParameterValue` _material_2 "Base Color" (`KismetMathLibrary.LinearColorLerp` (`self.Normal Color`) (`self.Warmup Color`) _warmup_time))
        (`MaterialInstanceDynamic.SetScalarParameterValue` _material_2 "Brightness" (`KismetMathLibrary.Lerp` (`self.Normal Brightness`) (`self.Warmup Brightness`) _warmup_time))
        (`ActorComponent.SetActive` _audio true false)
        (`AudioComponent.SetPitchMultiplier` _audio (`KismetMathLibrary.Lerp` (`self.Normal Pitch Multiplier`) (`self.Max Pitch Multiplier`) _warmup_time))
        (if (`self.Was Active`)
          (`self.Deactivate Interactions`)
          (set `self.Was Active` false)))
      (:`Finished`
        (if (== _direction 0)
          (`MaterialInstanceDynamic.SetVectorParameterValue` _material "Base Color" (`self.Active Color`))
          (`MaterialInstanceDynamic.SetScalarParameterValue` _material "Brightness" (`self.Active Brightness`))
          (set `self.Was Active` true)
          (`self.Activate Interactions`)
          (`GameplayStatics.PlaySoundAtLocation` "/Game/Audio/Sounds/Gem_Activate.Gem_Activate" (`SceneComponent.K2_GetComponentLocation` (`self.Diamond`)) (struct) 1.0 1.0 0.0 null null null null)
          (else
            (`ActorComponent.SetActive` (`self.Audio`) false false)))))))

(event `Deactivate`
  (if (`self.Active`)
    (set `self.Active` false)
    (goto _label :!via `Reverse`)))

(fn `Activate Interactions`
  (for _array_element (`self.Interactions`)
    (bind _asinteraction_door_bp (cast `/Game/Blueprints/Interaction_Door_bp` _array_element))
    (`/Game/Blueprints/Interaction_Door_bp.Activate` _asinteraction_door_bp self)))

(fn `Deactivate Interactions`
  (for _array_element (`self.Interactions`)
    (bind _asinteraction_door_bp (cast `/Game/Blueprints/Interaction_Door_bp` _array_element))
    (`/Game/Blueprints/Interaction_Door_bp.Deactivate` _asinteraction_door_bp self)))

(fn `UserConstructionScript`
  (set `self.Base Rotation` (`RotatingMovementComponent.RotationRate` (`self.RotatingMovement`)))
  (bind _returnvalue (`KismetMaterialLibrary.CreateDynamicMaterialInstance` (`PrimitiveComponent.GetMaterial` (`self.Diamond`) 0)))
  (bind _output_get (set `self.Material` _returnvalue))
  (bind _returnvalue_2 (`MaterialInstanceDynamic.K2_GetVectorParameterValue` _output_get "Base Color"))
  (set `self.Normal Color` _returnvalue_2)
  (bind _returnvalue_3 (`MaterialInstanceDynamic.K2_GetScalarParameterValue` _output_get "Brightness"))
  (set `self.Normal Brightness` _returnvalue_3)
  (`PrimitiveComponent.SetMaterial` (`self.Diamond`) 0 _output_get)
  (set `self.Normal Pitch Multiplier` (`AudioComponent.PitchMultiplier` (`self.Audio`))))