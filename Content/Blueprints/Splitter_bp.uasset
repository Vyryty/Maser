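; Splitter is an actor Blueprint that exposes a set of exit transforms; the file does not show what passes through it.
; Its construction script gathers the Arrow components parented under its StaticMesh into ExitPoints, so exits are defined by placing arrows in the component hierarchy.
; GetExitPoints returns the world transforms of those arrows.
; The event graph holds only disabled default events.
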(fn `Get Exit Points`
  (returns (`Exit Points` :type "Array of Transform Structure"))
  (locals (Exits :type "Array of Transform Structure"))
  (bind _exits (`local.Exits`))
  (for _array_element (`self.Exit Points`)
    (`KismetArrayLibrary.Array_Add` _exits (`SceneComponent.K2_GetComponentToWorld` _array_element)))
  (return _exits))

(fn `UserConstructionScript`
  (`parent.UserConstructionScript`)
  (for _array_element (`SceneComponent.GetChildrenComponents` (`self.StaticMesh`) true)
    (bind _asarrow_component (cast `ArrowComponent` _array_element))
    (`KismetArrayLibrary.Array_Add` (`self.Exit Points`) _asarrow_component)))