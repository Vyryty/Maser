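; Teleporter pad that sends overlapping Characters to a linked TargetTeleporter after a warm-up.
; While active, capsule overlaps fill an Interactors set and start a Delay-loop timer that aborts if the set empties.
; On completion, both pads deactivate for a cooldown before the move, so arrivals do not register at the destination.
; Each occupant keeps its offset from the capsule, applied to the target's ReceivingLocation cached in the Construction Script.
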(event `self.Capsule.OnComponentBeginOverlap`
  (params (OverlappedComponent :type "PrimitiveComponent Object Reference") (OtherActor :type "Actor Object Reference") (OtherComp :type "PrimitiveComponent Object Reference") (OtherBodyIndex :type Integer) (bFromSweep :type Boolean) (SweepResult :type "HitResult Structure (by ref)"))
  (cast `Character` OtherActor)
  (if (`self.Active`)
    (`BlueprintSetLibrary.Set_Add` (`self.Interactors`) OtherActor)
    (`self.Warm Up`)))

(event `self.Capsule.OnComponentEndOverlap`
  (params (OverlappedComponent :type "PrimitiveComponent Object Reference") (OtherActor :type "Actor Object Reference") (OtherComp :type "PrimitiveComponent Object Reference") (OtherBodyIndex :type Integer))
  (`BlueprintSetLibrary.Set_Remove` (`self.Interactors`) OtherActor))

(event `Warm Up`
  (if (and (not (`self.Warming Up`)) (`KismetSystemLibrary.IsValid` (`self.Target Teleporter`)))
    (set `self.Warming Up` true)
    (set `self.Timer` 0.0)
    (if (`BlueprintSetLibrary.Set_IsEmpty` (`self.Interactors`)) :!label _label
      (set `self.Warming Up` false)
      (else
        (bind _output_get (set `self.Timer` (+ (`self.Timer`) 0.1)))
        (if (>= _output_get (`self.Warmup`))
          (`self.Teleport`)
          (else
            (`KismetSystemLibrary.Delay` 0.1)
            (goto _label)))))))

(event `Deactivate`
  (set `self.Active` false)
  (`KismetSystemLibrary.Delay` (`self.Cooldown`))
  (set `self.Active` true)
  (set `self.Warming Up` false)
  (set `self.Timer` 0.0))

(fn `Teleport`
  (`self.Deactivate` self)
  (`self.Deactivate` (`self.Target Teleporter`))
  (bind _result (`BlueprintSetLibrary.Set_ToArray` (`self.Interactors`)))
  (for _array_element _result
    (`self.K2_SetActorLocation` _array_element (+ (`/Game/Blueprints/Teleporter_bp.Receiving Location` (`self.Target Teleporter`)) (- (`self.K2_GetActorLocation` _array_element) (`SceneComponent.K2_GetComponentLocation` (`self.Capsule`)))) false true)))

(fn `UserConstructionScript`
  (set `self.Receiving Location` (`SceneComponent.K2_GetComponentLocation` (`self.Capsule`))))