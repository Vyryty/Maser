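; Door Blueprint that swings open 90 degrees inward or outward on request and closes again, with audio for each action.
; OpenDoor and CloseDoor play or reverse one timeline, which lerps from the door's current rotation toward a target picked by the Opening and Outward flags.
; Opening sets Stuck, so a Sticky door ignores CloseDoor until Unstick clears the flag and immediately attempts the close.
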(event `Open Door`
  (params (Outward :type Boolean))
  (bind _door (`self.Door`))
  (bind _opening (`self.Opening`))
  (if (not (`self.Opening`))
    (set `self.Stuck` true)
    (set `self.Opening` true)
    (`AudioComponent.Play` (`self.Open`) 0.0)
    (bind (_direction _open_door) (`Timeline|Door Control` :!label _label)
      (:`Update`
        (`SceneComponent.K2_SetRelativeRotation` _door (`KismetMathLibrary.RLerp` (`SceneComponent.RelativeRotation` _door) (`KismetMathLibrary.SelectRotator` (`KismetMathLibrary.SelectRotator` (struct :`Yaw` 90.0) (struct :`Yaw` -90.0) Outward) (struct) _opening) (`KismetMathLibrary.SelectFloat` _open_door (- 1.0 _open_door) _opening)) false false)))))

(event `Close Door`
  (if (and (`self.Opening`) (or (not (`self.Sticky`)) (not (`self.Stuck`)))) :!label _label_2
    (set `self.Opening` false)
    (`AudioComponent.Play` (`self.Close`) 0.0)
    (goto _label :!via `Reverse`)))

(event `Unstick`
  (set `self.Stuck` false)
  (goto _label_2))

(fn `UserConstructionScript`)