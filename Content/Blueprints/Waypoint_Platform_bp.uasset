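; Moving platform that follows editable waypoints and can crush the player.
; The construction script copies Waypoints into the InterpToMovement component's control points and applies the Duration.
; Tick derives Velocity from the change in position each frame.
; When the Box begins overlapping Cello_bp while the platform's downward speed meets a small threshold, it defeats the player.
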(event `self.ReceiveBeginPlay`
  (set `self.Previous Position` (`self.K2_GetActorLocation`)))

(event `self.ReceiveTick`
  (params (DeltaSeconds :type "Float (single-precision)"))
  (bind _returnvalue (`self.K2_GetActorLocation`))
  (`parent.ReceiveTick` DeltaSeconds)
  (set `self.Velocity` (/ (- _returnvalue (`self.Previous Position`)) DeltaSeconds))
  (set `self.Previous Position` _returnvalue))

(event `self.Box.OnComponentBeginOverlap`
  (params (OverlappedComponent :type "PrimitiveComponent Object Reference") (OtherActor :type "Actor Object Reference") (OtherComp :type "PrimitiveComponent Object Reference") (OtherBodyIndex :type Integer) (bFromSweep :type Boolean) (SweepResult :type "HitResult Structure (by ref)"))
  (bind _ascello_bp (cast `/Game/Blueprints/Cello_bp` OtherActor))
  (if (<= (`KismetMathLibrary.Dot_VectorVector` (`self.Velocity`) (`KismetMathLibrary.Vector_Up`)) -0.75)
    (`/Game/Blueprints/Cello_bp.Defeat Player` _ascello_bp)))

(fn `UserConstructionScript`
  (bind _interptomovement (`self.InterpToMovement`))
  (`parent.UserConstructionScript`)
  (for (_array_element _array_index) (`self.Waypoints`)
    (`KismetArrayLibrary.Array_Set` (`InterpToMovementComponent.ControlPoints` _interptomovement) _array_index (make `InterpControlPoint` _array_element) true))
  (set `InterpToMovementComponent.Duration` (`self.Duration`) _interptomovement))