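; Pressure plate that activates linked doors and lasers when something overlaps its box, and deactivates them once its contact set is empty.
; A timeline lowers and raises the plate as its material switches between active and inactive.
; Press and release sounds start at an offset derived from timeline position, so interrupted moves resume mid-sound.
; Sticky plates stay down until Unstick clears the latch and rechecks contacts.
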(event `self.Box.OnComponentBeginOverlap`
  (params (OverlappedComponent :type "PrimitiveComponent Object Reference") (OtherActor :type "Actor Object Reference") (OtherComp :type "PrimitiveComponent Object Reference") (OtherBodyIndex :type Integer) (bFromSweep :type Boolean) (SweepResult :type "HitResult Structure (by ref)"))
  (bind _original_plate_position (`self.Original Plate Position`))
  (bind _audio (`self.Audio`))
  (`BlueprintSetLibrary.Set_Add` (`self.Contacts`) OtherComp)
  (set `self.Active` true)
  (`self.Activate Interactions`)
  (`PrimitiveComponent.SetMaterial` (`self.Plate`) 0 "/Game/Materials/Pressure_Plate_Active_inst.Pressure_Plate_Active_inst")
  (if (`self.Sticky`)
    (set `self.Stuck` true))
  (`AudioComponent.Stop` _audio)
  (`AudioComponent.SetSound` _audio "/Game/Audio/Sounds/Pressure_plate_down.Pressure_plate_down")
  (`AudioComponent.Play` _audio (`KismetMathLibrary.Lerp` 0.0 (`SoundBase.Duration` (`AudioComponent.Sound` (`self.Audio`))) (`KismetMathLibrary.SelectFloat` (- 1.0 (stale `self.Box.OnComponentBeginOverlap` _plate_position)) (stale `self.Box.OnComponentBeginOverlap` _plate_position) (== 0 (stale `self.Box.OnComponentBeginOverlap` _direction)))))
  (bind (_direction _plate_position) (`Timeline|Plate Control` :!label _label)
    (:`Update`
      (`SceneComponent.K2_SetRelativeLocation` (`self.Plate`) (`KismetMathLibrary.VLerp` _original_plate_position (+ _original_plate_position (0.0 0.0 -5.0)) _plate_position) false false))))

(event `self.Box.OnComponentEndOverlap`
  (params (OverlappedComponent :type "PrimitiveComponent Object Reference") (OtherActor :type "Actor Object Reference") (OtherComp :type "PrimitiveComponent Object Reference") (OtherBodyIndex :type Integer))
  (bind _contacts (`self.Contacts`))
  (bind _audio (`self.Audio`))
  (`BlueprintSetLibrary.Set_Remove` _contacts OtherComp)
  (bind _output_get (set `self.Active` (`BlueprintSetLibrary.Set_IsEmpty` _contacts) :!label _label_2))
  (if (and _output_get (not (`self.Stuck`)))
    (`self.Deactivate Interactions`)
    (`PrimitiveComponent.SetMaterial` (`self.Plate`) 0 "/Game/Materials/Pressure_Plate_Inactive_inst.Pressure_Plate_Inactive_inst")
    (`AudioComponent.Stop` _audio)
    (`AudioComponent.SetSound` _audio "/Game/Audio/Sounds/Pressure_plate_up.Pressure_plate_up")
    (`AudioComponent.Play` _audio (`KismetMathLibrary.Lerp` 0.0 (`SoundBase.Duration` (`AudioComponent.Sound` (`self.Audio`))) (`KismetMathLibrary.SelectFloat` (- 1.0 (stale `self.Box.OnComponentBeginOverlap` _plate_position)) (stale `self.Box.OnComponentBeginOverlap` _plate_position) (== 0 (stale `self.Box.OnComponentBeginOverlap` _direction)))))
    (goto _label :!via `Reverse`)))

(event `Unstick`
  (set `self.Stuck` false)
  (goto _label_2))

(fn `Activate Interactions`
  (for _array_element (`self.Interactions`)
    (bind _asinteraction_door_bp (cast `/Game/Blueprints/Interaction_Door_bp` _array_element)
      (:`then`
        (`/Game/Blueprints/Interaction_Door_bp.Activate` _asinteraction_door_bp self))
      (:`CastFailed`
        (bind _asactivatable_laser_bp (cast `/Game/Blueprints/Activatable_Laser_bp` _array_element))
        (`/Game/Blueprints/Activatable_Laser_bp.Activate` _asactivatable_laser_bp self)))))

(fn `Deactivate Interactions`
  (for _array_element (`self.Interactions`)
    (bind _asinteraction_door_bp (cast `/Game/Blueprints/Interaction_Door_bp` _array_element)
      (:`then`
        (`/Game/Blueprints/Interaction_Door_bp.Deactivate` _asinteraction_door_bp self))
      (:`CastFailed`
        (bind _asactivatable_laser_bp (cast `/Game/Blueprints/Activatable_Laser_bp` _array_element))
        (`/Game/Blueprints/Activatable_Laser_bp.Deactivate` _asactivatable_laser_bp self)))))

(fn `UserConstructionScript`
  (set `self.Original Plate Position` (`SceneComponent.RelativeLocation` (`self.Plate`))))