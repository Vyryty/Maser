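; Goal actor that ends the level when the Cello player character overlaps its capsule and loads the configured next level.
; Overlap calls WinLevel on the player and plays the DoorControl timeline, rotating the inner pod and turning the player's capsule 180 degrees in yaw.
; The timeline's update also feeds a WinDelay before opening the level, while its finish plays the victory sound at the outer pod.
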(event `self.Capsule.OnComponentBeginOverlap`
  (params (OverlappedComponent :type "PrimitiveComponent Object Reference") (OtherActor :type "Actor Object Reference") (OtherComp :type "PrimitiveComponent Object Reference") (OtherBodyIndex :type Integer) (bFromSweep :type Boolean) (SweepResult :type "HitResult Structure (by ref)"))
  (bind _player_rotation (`self.Player Rotation`))
  (bind _ascello_bp (cast `/Game/Blueprints/Cello_bp` OtherActor))
  (bind _capsulecomponent (`Character.CapsuleComponent` _ascello_bp))
  (set `self.Player Rotation` (`SceneComponent.K2_GetComponentRotation` _capsulecomponent))
  (`/Game/Blueprints/Cello_bp.Win Level` _ascello_bp)
  (bind (_direction _door_control) (`Timeline|Door Control`)
    (:`Update`
      (`SceneComponent.K2_SetRelativeRotation` (`self.Inner Pod`) (`KismetMathLibrary.RLerp` (struct) (struct :`Yaw` 180.0) _door_control) false false)
      (`SceneComponent.K2_SetWorldRotation` _capsulecomponent (`KismetMathLibrary.RLerp` _player_rotation (`KismetMathLibrary.MakeRotator` (.roll _player_rotation) (.pitch _player_rotation) (+ (.yaw _player_rotation) 180.0)) _door_control) false false)
      (`KismetSystemLibrary.Delay` (`self.Win Delay`))
      (bind _level (`self.Level`)
        (:`then`
          (`GameplayStatics.OpenLevelBySoftObjectPtr` _level))
        (:`else`)))
    (:`Finished`
      (`GameplayStatics.PlaySoundAtLocation` "/Game/Audio/Sounds/Victory.Victory" (`SceneComponent.K2_GetComponentLocation` (`self.Outer Pod`)) (struct) 1.0 1.0 0.0 null null null null))))

(fn `UserConstructionScript`)